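; BP_Car is a player-controlled car built on Character movement, driven through Enhanced Input.
; On BeginPlay it adds the third-person movement mapping context, and look input feeds controller yaw and pitch.
; Movement input follows the mesh's right and forward vectors rather than the control rotation.
; Full reverse input zeroes the CharacterMovement rotation rate, and any other movement input restores it, so movement-driven turning stops while backing up.
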(event `self.ReceiveBeginPlay`
  ;[0.159 0.53 0.6906] Event Begin
  (bind _asplayer_controller (cast `PlayerController` (`self.GetController`)))
  (`EnhancedInputSubsystemInterface.AddMappingContext` (pcsubsystem `EnhancedInputLocalPlayerSubsystem` _asplayer_controller) "/Game/Input/IMC_TPMovement.IMC_TPMovement" 0 (struct)))

(event `EnhancedInput|/Game/Input/Action/IA_Movement`
  (params (ActionValue :type "Vector2D Structure") (ElapsedSeconds :type "Float (double-precision)") (TriggeredSeconds :type "Float (double-precision)") (InputAction :type "InputAction Object Reference" :default "/Game/Input/Action/IA_Movement.IA_Movement"))
  (bind _mesh (`self.Mesh`))
  (bind _charactermovement (`self.CharacterMovement`))
  ;[1 0.572 0.6746] Movement
  (:`Triggered`
    (`self.AddMovementInput` (`SceneComponent.GetRightVector` _mesh) ActionValue_X)
    (`self.AddMovementInput` (`SceneComponent.GetForwardVector` _mesh) ActionValue_Y)
    (if (<= ActionValue_Y -1.0)
      (set `CharacterMovementComponent.RotationRate` (struct) _charactermovement)
      (else
        (set `CharacterMovementComponent.RotationRate` (struct :`Yaw` 90.0) _charactermovement)))))

(event `EnhancedInput|/Game/Input/Action/IA_Look`
  (params (ActionValue :type "Vector2D Structure") (ElapsedSeconds :type "Float (double-precision)") (TriggeredSeconds :type "Float (double-precision)") (InputAction :type "InputAction Object Reference" :default "/Game/Input/Action/IA_Look.IA_Look"))
  ;[1 0.572 0.6746] Look around
  (:`Triggered`
    (`self.AddControllerYawInput` ActionValue_X)
    (`self.AddControllerPitchInput` ActionValue_Y)))

(fn `UserConstructionScript`)